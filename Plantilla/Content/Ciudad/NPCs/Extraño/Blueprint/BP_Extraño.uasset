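; BP_Extraño is the Stranger NPC in the city, an actor that can be teleported into place in front of the player and sent back.
; On BeginPlay it caches its original location and rotation.
; AparecerFrenteAlJugador snaps it to the PosicionExtraño reference's transform rather than computing one from the camera.
; RegresarAPosicionOriginal restores the cached transform and destroys the BP_EventoDialogo actor found in the level.
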(event Custom|AparecerFrenteAlJugador
  (bind _posicionextraño (Variables|Default|GetPosicionExtraño))
  (bind _rootcomponent (Variables|/Script/Engine.Actor|GetRootComponent _posicionextraño))
  (bind _returnvalue (Transformation|GetWorldLocation _rootcomponent))
  (Transformation|SetActorLocationAndRotation (Math|Vector|MakeVector (.x _returnvalue) (.y _returnvalue) (.z _returnvalue)) (Transformation|GetWorldRotation (Variables|/Script/Engine.Actor|GetRootComponent _posicionextraño))))

(event Custom|RegresarAPosicionOriginal
  (Transformation|SetActorLocationAndRotation (Variables|Default|GetPosicionOriginal) (Variables|Default|GetRotacionOriginal))
  (bind _returnvalue (Actor|GetActorOfClass "/Game/Programacion/BP_EventoDialogo.BP_EventoDialogo_C"))
  (Actor|DestroyActor _returnvalue))

(event EventBeginPlay
  (Variables|Default|SetPosicionOriginal (Transformation|GetActorLocation))
  (Variables|Default|SetRotacionOriginal (Transformation|GetActorRotation)))

(event Collision|EventActorBeginOverlap
  (params (OtherActor :type Actor%20Object%20Reference)))

(event EventTick
  (params (DeltaSeconds :type Float%20%28single-precision%29)))

(fn ConstructionScript)