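; BP_Mapa is a grabbable VR map that rests at the player's right-hand-side socket (SocketDerecha), treated as a belt slot.
; On BeginPlay it caches the VRPawn, then moves its Plane to that socket's location every tick until first grabbed.
; Grabbing clears the on-belt flag, which is never set again; dropping attaches the Plane to the socket, snapping location and rotation while keeping world scale.
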(event OnGrabbed(GrabComponent)
  (Variables|Default|SetEstaEnElCinturon? false))

(event OnDropped(GrabComponent)
  (Transformation|AttachComponentToComponent (Variables|Default|GetPlane) (Variables|/Game/VRTemplate/Blueprints/VRPawn.VRPawn_C|GetSocketDerecha (Variables|Default|GetRef_PJ)) "None" "SnapToTarget" "SnapToTarget" "KeepWorld" true))

(event EventBeginPlay
  (bind _asvrpawn (Utilities|Casting|CastToVRPawn (Game|Player|GetPlayerPawn 0)))
  (Variables|Default|SetRef_PJ _asvrpawn)
  (Transformation|SetWorldLocation (Variables|Default|GetPlane) (Transformation|GetWorldLocation (Variables|/Game/VRTemplate/Blueprints/VRPawn.VRPawn_C|GetSocketDerecha (Variables|Default|GetRef_PJ))) false false)
  (Variables|Default|SetEstaEnElCinturon? true))

(event Collision|EventActorBeginOverlap
  (params (OtherActor :type Actor%20Object%20Reference)))

(event EventTick
  (params (DeltaSeconds :type Float%20%28single-precision%29))
  (if (Variables|Default|GetEstaEnElCinturon?)
    (Transformation|SetWorldLocation (Variables|Default|GetPlane) (Transformation|GetWorldLocation (Variables|/Game/VRTemplate/Blueprints/VRPawn.VRPawn_C|GetSocketDerecha (Variables|Default|GetRef_PJ))) false false)))

(fn ConstructionScript)